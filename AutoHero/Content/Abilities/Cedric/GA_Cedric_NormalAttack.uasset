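; Cedric's normal attack ability, which chooses between two attack montages based on a charge Gameplay Effect.
; Activation runs the parent logic, then applies the normal attack charge effect to the owner.
; The GetMontageToPlay function counts that effect on the owner, returning the first attack montage when none is found and the second otherwise.
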(event `self.K2_ActivateAbility`
  (`parent.K2_ActivateAbility`)
  (`self.BP_ApplyGameplayEffectToOwner` "/Game/Abilities/Cedric/GE_CedricNormalAttack_Charge.GE_CedricNormalAttack_Charge_C"))

(event `self.K2_OnEndAbility`
  (params (bWasCancelled :type Boolean))
  (`parent.K2_OnEndAbility` bWasCancelled))

(fn `GetMontageToPlay`
  (returns (OutMontageToPlay :type "AnimMontage Object Reference"))
  (bind _returnvalue_owneractor (break `GameplayAbilityActorInfo` (`self.GetActorInfo`)))
  (if (== (`AbilitySystemComponent.GetGameplayEffectCount` (`AbilitySystemBlueprintLibrary.GetAbilitySystemComponent` _returnvalue_owneractor) "/Game/Abilities/Cedric/GE_CedricNormalAttack_Charge.GE_CedricNormalAttack_Charge_C" null true) 0)
    (return "/Game/Characters/Cedric/Montages/AM_Cedric_Attack1.AM_Cedric_Attack1")
    (else
      (return "/Game/Characters/Cedric/Montages/ANM_Cedric_Attack2.ANM_Cedric_Attack2"))))