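; Gameplay ability for Elara's Rain Arrow, which drops a projectile from the sky onto her current enemy.
; On activation it applies a mana cost effect to the owner, plays the montage and waits once for the fire gameplay event.
; That event reads EnemyToAttack from the owner's blackboard and spawns the arrow high above that unit, pitched straight down.
; EndAbility is present but unconnected, so the ability never ends itself.
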(event `self.K2_ActivateAbility`
  (bind (_returnvalue_owneractor _returnvalue_avataractor _returnvalue_playercontroller _returnvalue_abilitysystemcomponent _returnvalue_skeletalmeshcomponent) (break `GameplayAbilityActorInfo` (`self.GetActorInfo`)))
  (`self.BP_ApplyGameplayEffectToOwner` "/Game/Abilities/Elara/RainArrow/GE_Elara_RainArrow_ManaCost.GE_Elara_RainArrow_ManaCost_C")
  (`|PlayMontage` _returnvalue_skeletalmeshcomponent "/Game/Characters/Elara/Montage/AM_Elara_RainArrow.AM_Elara_RainArrow"
    (:`then`
      (bind (_asynctaskproxy _payload) (`AbilityTask_WaitGameplayEvent.WaitGameplayEvent` (struct :`TagName` "char.elara.rainarrow.fire") null true)
        (:`then`
          (set `self.Async Task` _asynctaskproxy))
        (:`EventReceived`
          (bind _asbase_unit (cast `BaseUnit` (`self.GetOwningActorFromActorInfo`))
            (:`then`
              (bind _asbase_unit_2 (cast `BaseUnit` (`BlackboardComponent.GetValueAsObject` (`AIBlueprintHelperLibrary.GetBlackboard` _asbase_unit) "EnemyToAttack"))
                (:`then`
                  (`|SpawnActorFromClass` "/Game/Blueprints/Projectiles/BP_ElaraProjectile_RainArrow.BP_ElaraProjectile_RainArrow_C" (`KismetMathLibrary.MakeTransform` (+ (`Actor.K2_GetActorLocation` _asbase_unit_2) (0.0 0.0 5000.0)) (struct :`Pitch` -90.0)) "AlwaysSpawn" "MultiplyWithRoot" null 3000.0 0.0 _asbase_unit null))
                (:`CastFailed`
                  (`KismetSystemLibrary.PrintText` "Target Not Found"))))
            (:`CastFailed`
              (`KismetSystemLibrary.PrintString` "CAST FAILED!!" true true (struct :`R` 1.0 :`B` 0.023943 :`A` 1.0)))))))))