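; Base projectile Blueprint that carries an owner and target unit and can home in on that target.
; Construction copies Speed and Gravity into the projectile movement component.
; Homing activation points velocity at the target on the horizontal plane, with a debug print, then sets the target's root as homing component.
; BanishUnitBP has the owner's ability system apply Faye's imprison crowd-control effect to a given unit.
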(fn `Activate Homing Target`
  (`/Engine/EditorBlueprintResources/StandardMacros.IsValid` (`self.TargetUnit`)
    (:`Is Valid`
      (`/Engine/EditorBlueprintResources/StandardMacros.IsValid` (`ProjectileMovementComponent.HomingTargetComponent` (`self.ProjectileMovementComponent`))
        (:`Is Valid`
          _)
        (:`Is Not Valid`
          _))
      (`self.RotateToTarget`)
      (set `ProjectileMovementComponent.HomingTargetComponent` (`Actor.RootComponent` (`self.TargetUnit`)) (`self.ProjectileMovementComponent`)))))

(fn `BanishUnitBP`
  (params (BaseUnit :type "/Game/Blueprints/Units/BP_BaseUnit Object Reference"))
  (`AbilitySystemComponent.BP_ApplyGameplayEffectToTarget` :`self` (`BaseUnit.AbilitySystemComponent` (`self.OwnerUnit`)) :`GameplayEffectClass` "/Game/Blueprints/Abilities/Faye/Imprison/GE_Faye_Imprison_CC.GE_Faye_Imprison_CC_C" :`Target` (`BaseUnit.AbilitySystemComponent` BaseUnit)))

(fn `OnRep_OwnerUnit`)

(fn `RotateToTarget`
  (`/Engine/EditorBlueprintResources/StandardMacros.IsValid` (`self.TargetUnit`)
    (:`Is Valid`
      (`KismetSystemLibrary.PrintText` "Rotate Projectile Toward Target")
      (set `MovementComponent.Velocity` (`KismetMathLibrary.MakeVector` (.x (* (`KismetMathLibrary.GetDirectionUnitVector` (`self.K2_GetActorLocation`) (`self.K2_GetActorLocation` (`self.TargetUnit`))) (`self.Speed`))) (.y (* (`KismetMathLibrary.GetDirectionUnitVector` (`self.K2_GetActorLocation`) (`self.K2_GetActorLocation` (`self.TargetUnit`))) (`self.Speed`)))) (`self.ProjectileMovementComponent`)))))

(fn `UserConstructionScript`
  (set `ProjectileMovementComponent.InitialSpeed` (`self.Speed`) (`self.ProjectileMovementComponent`))
  (set `ProjectileMovementComponent.MaxSpeed` (`self.Speed`) (`self.ProjectileMovementComponent`))
  (set `ProjectileMovementComponent.ProjectileGravityScale` (`self.Gravity`) (`self.ProjectileMovementComponent`)))