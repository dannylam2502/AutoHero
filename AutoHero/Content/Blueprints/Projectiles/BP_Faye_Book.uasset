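; Faye's book projectile, which damages and banishes units on teams other than its owner's.
; FindTargets gathers every BP_BaseUnit in the level whose team differs from OwnerUnit's, with no range check.
; FindAndBanishUnits applies the GE_Faye_Imprison_Damage gameplay effect from the owner's ability system component to each target, then calls BanishUnit on it.
; The event graph only forwards BeginPlay to the parent, so FindAndBanishUnits is not triggered within this Blueprint.
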(event `self.ReceiveBeginPlay`
  (`parent.ReceiveBeginPlay`))

(fn `FindAndBanishUnits`
  (bind _targets (`self.FindTargets`))
  (for _array_element _targets
    (`AbilitySystemComponent.BP_ApplyGameplayEffectToTarget` :`self` (`BaseUnit.AbilitySystemComponent` (`self.OwnerUnit`)) :`GameplayEffectClass` "/Game/Blueprints/Abilities/Faye/Imprison/GE_Faye_Imprison_Damage.GE_Faye_Imprison_Damage_C" :`Target` (`BaseUnit.AbilitySystemComponent` _array_element))
    (`self.BanishUnit` _array_element)))

(fn `FindTargets`
  (returns (Targets :type "Array of /Game/Blueprints/Units/BP_BaseUnit Object Reference"))
  (locals (Result :type "Array of /Game/Blueprints/Units/BP_BaseUnit Object Reference"))
  (bind _outactors (`GameplayStatics.GetAllActorsOfClass` "/Game/Blueprints/Units/BP_BaseUnit.BP_BaseUnit_C"))
  (for _array_element _outactors
    (if (`|EnumInequality` (`BaseUnit.ETeam` _array_element) (`BaseUnit.ETeam` (`self.OwnerUnit`)))
      (`KismetArrayLibrary.Array_Add` (`local.Result`) _array_element)))
  (return (`local.Result`)))

(fn `UserConstructionScript`
  (`parent.UserConstructionScript`))