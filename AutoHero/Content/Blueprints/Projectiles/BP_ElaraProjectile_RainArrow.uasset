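; Rain arrow projectile for Elara that deals area damage where it hits, using the Gameplay Ability System.
; On Hit, it applies the rain arrow damage effect from the owner's ability system to every BaseUnit overlapping its sphere, without a team check.
; It then plays Elara's hit gameplay cue slightly above the impact point and destroys itself.
; An older team-filtered hit path remains but is disconnected.
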(event `self.ReceiveHit`
  (params (MyComp :type "PrimitiveComponent Object Reference") (Other :type "Actor Object Reference") (OtherComp :type "PrimitiveComponent Object Reference") (bSelfMoved :type Boolean) (HitLocation :type "Vector Structure") (HitNormal :type "Vector Structure") (NormalImpulse :type "Vector Structure") (Hit :type "HitResult Structure (by ref)"))
  (`KismetSystemLibrary.PrintText` "Elara Rain Arrow Hit Plane")
  (for _array_element (`PrimitiveComponent.GetOverlappingActors` (`self.SphereComponent`) "/Script/AutoHero.BaseUnit")
    (bind _asbase_unit (cast `BaseUnit` _array_element))
    (`KismetSystemLibrary.PrintText` (`KismetTextLibrary.Conv_StringToText` (`KismetStringLibrary.Concat_StrStr` "Overlapping: " (`KismetSystemLibrary.GetDisplayName` _asbase_unit))))
    (`AbilitySystemComponent.BP_ApplyGameplayEffectToTarget` :`self` (`BaseUnit.AbilitySystemComponent` (`self.OwnerUnit`)) :`GameplayEffectClass` "/Game/Abilities/Elara/RainArrow/GE_Elara_RainArrow_Damage.GE_Elara_RainArrow_Damage_C" :`Target` (`AbilitySystemBlueprintLibrary.GetAbilitySystemComponent` _asbase_unit)))
  ;[1 1 1] Out Of Loop
  (`GameplayCueFunctionLibrary.ExecuteGameplayCueOnActor` (`self.OwnerUnit`) (struct :`TagName` "Gameplaycue.Elara.NMAtt.Hit") (`AbilitySystemBlueprintLibrary.MakeGameplayCueParameters` 0.0 0.0 (struct) (struct) (struct) (struct) (struct) (+ HitLocation (0.0 0.0 100.0))))
  (`self.K2_DestroyActor`))

(fn `UserConstructionScript`
  (`parent.UserConstructionScript`))