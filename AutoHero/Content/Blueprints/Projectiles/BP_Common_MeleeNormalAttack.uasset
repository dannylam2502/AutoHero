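; A shared melee normal-attack projectile actor that resolves a unit's hit instantly on spawn rather than travelling.
; On BeginPlay, if both owner and target units are valid, it applies the normal-attack damage GameplayEffect from the owner's ability system to the target's.
; It then fires a hit GameplayCue on the owner at the target's location, using an Elara-specific tag despite the common name, and destroys itself.
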(event `self.ReceiveBeginPlay`
  (bind _targetunit (`self.TargetUnit`))
  (`parent.ReceiveBeginPlay`)
  (`/Engine/EditorBlueprintResources/StandardMacros.IsValid` (`self.OwnerUnit`)
    (:`Is Valid`
      (`/Engine/EditorBlueprintResources/StandardMacros.IsValid` _targetunit
        (:`Is Valid`
          (`AbilitySystemComponent.BP_ApplyGameplayEffectToTarget` :`self` (`BaseUnit.AbilitySystemComponent` (`self.OwnerUnit`)) :`GameplayEffectClass` "/Game/Blueprints/Abilities/Common/GE_UnitNormalAttack_Damage.GE_UnitNormalAttack_Damage_C" :`Target` (`BaseUnit.AbilitySystemComponent` _targetunit)) ; Damage
          (`GameplayCueFunctionLibrary.ExecuteGameplayCueOnActor` (`self.OwnerUnit`) (struct :`TagName` "Gameplaycue.Elara.NMAtt.Hit") (`AbilitySystemBlueprintLibrary.MakeGameplayCueParameters` 0.0 0.0 (struct) (struct) (struct) (struct) (struct) (`self.K2_GetActorLocation` (`self.TargetUnit`))))
          (`self.K2_DestroyActor`))))))

(fn `UserConstructionScript`
  (`parent.UserConstructionScript`))