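; Projectile Blueprint for Cocu's normal attack that damages a single assigned target unit.
; On overlapping TargetUnit, it applies GE_UnitNormalAttack_Damage from the owner's ability system to the target's, fires Elara's normal-attack hit GameplayCue there, and destroys itself.
; Other overlaps are ignored, and Tick adds only an empty target validity check after the parent call, so any movement is left to the parent.
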(event `self.ReceiveBeginPlay`
  (`parent.ReceiveBeginPlay`))

(event `self.ReceiveTick`
  (params (DeltaSeconds :type "Float (single-precision)"))
  (`parent.ReceiveTick` DeltaSeconds)
  (`/Engine/EditorBlueprintResources/StandardMacros.IsValid` (`self.TargetUnit`)))

(event `self.ReceiveActorBeginOverlap`
  (params (OtherActor :type "Actor Object Reference"))
  (bind _targetunit (`self.TargetUnit`))
  (if (== OtherActor (`self.TargetUnit`))
    (`KismetSystemLibrary.PrintText` "Received Event Hit" true true (struct :`R` 1.0 :`B` 0.07119 :`A` 1.0))
    (`AbilitySystemComponent.BP_ApplyGameplayEffectToTarget` :`self` (`AbilitySystemBlueprintLibrary.GetAbilitySystemComponent` (`self.OwnerUnit`)) :`GameplayEffectClass` "/Game/Blueprints/Abilities/Common/GE_UnitNormalAttack_Damage.GE_UnitNormalAttack_Damage_C" :`Target` (`AbilitySystemBlueprintLibrary.GetAbilitySystemComponent` (`self.TargetUnit`)))
    (`GameplayCueFunctionLibrary.ExecuteGameplayCueOnActor` _targetunit (struct :`TagName` "Gameplaycue.Elara.NMAtt.Hit") (`AbilitySystemBlueprintLibrary.MakeGameplayCueParameters` 0.0 0.0 (struct) (struct) (struct) (struct) (struct) (`self.K2_GetActorLocation` _targetunit)))
    (`self.K2_DestroyActor`)))

(fn `UserConstructionScript`
  (`parent.UserConstructionScript`))