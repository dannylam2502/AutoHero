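; Pinwheel skill actor for Titus that deals area damage around its owning unit while the skill is active.
; Each Tick it snaps to the owner's location and destroys itself once the owner's Activating gameplay effect is gone.
; Gameplay effect counts act as the damage clock: whenever the Charge count exceeds the last recorded one, DealDamage applies the damage effect to enemy-team units overlapping the sphere.
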(event `self.ReceiveTick`
  (params (DeltaSeconds :type "Float (single-precision)"))
  (bind _ownerunit (`self.OwnerUnit`))
  (bind _returnvalue (`AbilitySystemComponent.GetGameplayEffectCount` (`BaseUnit.AbilitySystemComponent` (`self.OwnerUnit`)) "/Game/Blueprints/Abilities/Titus/Spin/GE_Titus_Pinwheel_Charge.GE_Titus_Pinwheel_Charge_C" null true))
  (`/Engine/EditorBlueprintResources/StandardMacros.IsValid` _ownerunit
    (:`Is Valid`
      (`self.K2_SetActorLocation` (`self.K2_GetActorLocation` _ownerunit)) ; Snap To Unit's position
      (if (> (`AbilitySystemComponent.GetGameplayEffectCount` (`BaseUnit.AbilitySystemComponent` (`self.OwnerUnit`)) "/Game/Blueprints/Abilities/Titus/Spin/GE_Titus_Pinwheel_Activating.GE_Titus_Pinwheel_Activating_C" null true) 0)
        (if (> _returnvalue (`self.LastEffectCount`))
          (set `self.LastEffectCount` _returnvalue)
          (`self.DealDamage`))
        (else
          (`self.K2_DestroyActor`))))))

(fn `DealDamage`
  (for _array_element (`PrimitiveComponent.GetOverlappingActors` (`self.SphereComponent`) "/Game/Blueprints/Units/BP_BaseUnit.BP_BaseUnit_C")
    ;[1 1 1] Loop Body Block, only deal damage to enemies
    (bind _asbp_unit (cast `/Game/Blueprints/Units/BP_BaseUnit` _array_element))
    (if (`|EnumInequality` (`BaseUnit.ETeam` _asbp_unit) (`BaseUnit.ETeam` (`self.OwnerUnit`)))
      (`AbilitySystemComponent.BP_ApplyGameplayEffectToTarget` :`self` (`BaseUnit.AbilitySystemComponent` (`self.OwnerUnit`)) :`GameplayEffectClass` "/Game/Blueprints/Abilities/Titus/Spin/GE_Titus_Pinwheel_Damage.GE_Titus_Pinwheel_Damage_C" :`Target` (`AbilitySystemBlueprintLibrary.GetAbilitySystemComponent` _asbp_unit)))))

(fn `UserConstructionScript`
  (`parent.UserConstructionScript`))