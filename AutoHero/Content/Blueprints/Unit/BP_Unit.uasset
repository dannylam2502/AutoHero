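; BP_Unit is a unit actor whose skeletal mesh and anim class come from its DT_Units data table row at construction.
; Each tick it smoothly rotates toward its velocity direction while moving.
; SetFocused toggles a custom-depth stencil highlight on the mesh, and SetDragState raises the mesh while dragged and lowers it on release, leaving the actor's own location untouched.
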(event `self.ReceiveActorBeginOverlap`
  (params (OtherActor :type "Actor Object Reference")))

(event `self.ReceiveTick`
  (params (DeltaSeconds :type "Float (single-precision)"))
  (`self.RotateTowardsMovement`))

(event `self.SkeletalMesh.OnBeginCursorOver`
  (params (TouchedComponent :type "PrimitiveComponent Object Reference")))

(event `self.SkeletalMesh.OnEndCursorOver`
  (params (TouchedComponent :type "PrimitiveComponent Object Reference")))

(fn `RotateTowardsMovement`
  (bind _returnvalue (`self.GetVelocity`))
  (bind _returnvalue_2 (`self.K2_GetActorLocation`))
  (if true
    (if (> (`KismetMathLibrary.VSize` _returnvalue) 0.0)
      (`self.K2_SetActorRotation` (`KismetMathLibrary.RInterpTo` (`self.K2_GetActorRotation`) (`KismetMathLibrary.FindLookAtRotation` _returnvalue_2 (+ (* _returnvalue (100.0 100.0 100.0)) _returnvalue_2)) (`GameplayStatics.GetWorldDeltaSeconds`) (`self.RotationSpeed`))))))

(fn `SetDragState`
  (params (bEnabled :type Boolean))
  (`self.SetMeshRelativeZState` bEnabled))

(fn `SetFocused`
  (params (bFocused :type Boolean))
  (bind _skeletalmesh (`self.SkeletalMesh`))
  (if bFocused
    (`KismetSystemLibrary.PrintString` "On Begin Cursor Over Skeletal Mesh")
    (`PrimitiveComponent.SetRenderCustomDepth` _skeletalmesh true)
    (`PrimitiveComponent.SetCustomDepthStencilValue` _skeletalmesh 250)
    (else
      (`PrimitiveComponent.SetRenderCustomDepth` _skeletalmesh false))))

(fn `SetMeshRelativeZState`
  (params (Dragged :type Boolean))
  (`KismetSystemLibrary.PrintString` "Set Mesh Relative State")
  (if Dragged
    (`SceneComponent.K2_SetRelativeLocation` (`self.SkeletalMesh`) (`KismetMathLibrary.MakeVector` 0.0 0.0 200.0) false false)
    (else
      (`SceneComponent.K2_SetRelativeLocation` (`self.SkeletalMesh`) (`KismetMathLibrary.MakeVector` 0.0 0.0 -50.0) false false))))

(fn `SetupCosmetics`
  (bind _skeletalmesh (`self.SkeletalMesh`))
  (bind _returnvalue (`|GetDataTableRow` "/Game/Data/DT_Units.DT_Units" (`.RowName` (break `DataTableRowHandle` (`self.UnitRow`))))
    (:`then`
      (bind (_name _skeletalmesh_2 _animinstance) (break `/Game/Blueprints/Unit/Utils/FUnit` _returnvalue))
      (`SkeletalMeshComponent.SetSkeletalMeshAsset` _skeletalmesh _skeletalmesh_2)
      (`SkeletalMeshComponent.SetAnimInstanceClass` _skeletalmesh _animinstance))))

(fn `UserConstructionScript`
  (`self.SetupCosmetics`))