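; BP_Elara_Two is an Elara unit Blueprint that adds the ranged normal attack.
; NormalAttackShoot reads EnemyToAttack from its controller's Blackboard and casts it to BaseUnit, stopping if the cast fails.
; It then spawns BP_ElaraProjectile_NormalAttack at the unit's location, passing that target and itself as owner.
; The construction script only calls the parent, and the other event nodes are disabled stubs.
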(event `Event NormalAttack Shoot`
  (bind _asbase_unit (cast `BaseUnit` (`BlackboardComponent.GetValueAsObject` (`AIBlueprintHelperLibrary.GetBlackboard` (`self.GetController`)) "EnemyToAttack")))
  (`|SpawnActorFromClass` "/Game/Blueprints/Projectiles/BP_ElaraProjectile_NormalAttack.BP_ElaraProjectile_NormalAttack_C" (`KismetMathLibrary.Conv_VectorToTransform` (`self.K2_GetActorLocation` self)) "Undefined" "MultiplyWithRoot" null _asbase_unit 700.0 0.0 self null))

(fn `UserConstructionScript`
  (`parent.UserConstructionScript`))