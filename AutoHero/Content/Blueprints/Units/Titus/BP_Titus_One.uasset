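; BP_Titus_One is a Titus unit Blueprint that defines the projectile used for its normal attack.
; SpawnNMAttProjectile spawns the shared BP_Common_MeleeNormalAttack at the given transform's location and rotation, passing along the owner and target units.
; The melee attack thus goes through the projectile spawn path.
; The event graph holds only disabled default events, and the construction script just calls its parent.
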(fn `SpawnNMAttProjectile`
  (params (OwnerUnit :type "BaseUnit Object Reference") (TargetUnit :type "BaseUnit Object Reference") (SpawnTransform :type "Transform Structure") (Instigator :type "Pawn Object Reference"))
  (`self.SpawnProjectile` self "/Game/Blueprints/Projectiles/BP_Common_MeleeNormalAttack.BP_Common_MeleeNormalAttack_C" (.location SpawnTransform) (.rotation SpawnTransform) 0.0 0.0 false OwnerUnit TargetUnit))

(fn `UserConstructionScript`
  (`parent.UserConstructionScript`))