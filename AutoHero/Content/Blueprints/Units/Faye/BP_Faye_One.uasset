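; BP_Faye_One is the unit Blueprint for Faye, defining her ultimate cast and normal-attack projectile.
; The ultimate start event prints a message, spawns a BP_Faye_Book projectile at her location with her as owner, then calls FindAndBanishUnits on it.
; SpawnNMAttProjectile reuses Elara's normal-attack projectile, spawning it toward the target unit and activating homing.
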(event `self.EventUltimateStartCast`
  (`KismetSystemLibrary.PrintString` "Faye Ultimate Cast")
  (bind _returnvalue (`self.SpawnProjectile` self "/Game/Blueprints/Projectiles/BP_Faye_Book.BP_Faye_Book_C" (`self.K2_GetActorLocation`) (struct) 0.0 0.0 false self null))
  (bind _asbp_faye_book (cast `/Game/Blueprints/Projectiles/BP_Faye_Book` _returnvalue))
  (`/Game/Blueprints/Projectiles/BP_Faye_Book.FindAndBanishUnits` _asbp_faye_book))

(fn `SpawnNMAttProjectile`
  (params (OwnerUnit :type "BaseUnit Object Reference") (TargetUnit :type "BaseUnit Object Reference") (SpawnTransform :type "Transform Structure") (Instigator :type "Pawn Object Reference"))
  (bind _returnvalue (`self.SpawnProjectile` OwnerUnit "/Game/Blueprints/Projectiles/BP_ElaraProjectile_NormalAttack.BP_ElaraProjectile_NormalAttack_C" (.location SpawnTransform) (struct) 700.0 0.0 true OwnerUnit TargetUnit))
  (bind _asbp_base_projectile (cast `/Game/Blueprints/Projectiles/BP_BaseProjectile` _returnvalue))
  (`/Game/Blueprints/Projectiles/BP_BaseProjectile.Activate Homing Target` _asbp_base_projectile))

(fn `UserConstructionScript`
  (`parent.UserConstructionScript`))