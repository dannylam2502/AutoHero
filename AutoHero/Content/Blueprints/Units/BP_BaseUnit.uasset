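; Base unit Blueprint for combat units that can be highlighted and dragged, with mesh and anim class set from a data table row.
; Normal attacks spawn a projectile at the Blackboard's EnemyToAttack, while Pinwheel applies a GAS effect and spawns a skill actor without setting its owner.
; Received damage goes through MulticastDamageReceived to spawn floating damage text.
; Tick turns the unit toward its velocity; focus uses custom depth, and dragging raises the mesh.
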(event `EventUltimateStartCast`
  (`KismetSystemLibrary.PrintString` "BP Unit Event Ultimate Start Cast"))

(event `Event Pinwheel Activate`
  (`AbilitySystemComponent.BP_ApplyGameplayEffectToSelf` :`self` (`self.AbilitySystemComponent`) :`GameplayEffectClass` "/Game/Blueprints/Abilities/Titus/Spin/GE_Titus_Pinwheel_Activating.GE_Titus_Pinwheel_Activating_C")
  (bind _returnvalue (`|SpawnActorFromClass` "/Game/Blueprints/Projectiles/BP_Skill_Pinwheel.BP_Skill_Pinwheel_C" (`KismetMathLibrary.Conv_VectorToTransform` (`self.K2_GetActorLocation`)) "Undefined" "MultiplyWithRoot" null 0.0 0.0 null)))

(event `self.ReceiveBeginPlay`)

(event `self.ReceiveActorBeginOverlap`
  (params (OtherActor :type "Actor Object Reference")))

(event `self.ReceiveTick`
  (params (DeltaSeconds :type "Float (single-precision)"))
  (`self.RotateTowardsMovement`))

(event `Event Fire Normal Attack`
  (bind _returnvalue (`AIBlueprintHelperLibrary.GetBlackboard` (`self.GetController`)))
  (`/Engine/EditorBlueprintResources/StandardMacros.IsValid` _returnvalue
    (:`Is Valid`
      (bind _asbase_unit (cast `BaseUnit` (`BlackboardComponent.GetValueAsObject` _returnvalue "EnemyToAttack")))
      (`self.SpawnNMAttProjectile` self _asbase_unit (`KismetMathLibrary.Conv_VectorToTransform` (`self.K2_GetActorLocation` self))))
    (:`Is Not Valid`
      (`KismetSystemLibrary.PrintString` "Event Fire Normal Attack BlackBoard Target No Valid"))))

(event `self.OnDamageReceived`
  (params (InInstigator :type "Actor Object Reference") (InCauser :type "Actor Object Reference") (InTags :type "GameplayTagContainer Structure (by ref)") (InDamage :type "Float (single-precision)"))
  (`self.MulticastDamageReceived` InInstigator InCauser InTags InDamage)
  (`KismetSystemLibrary.PrintString` (`KismetStringLibrary.Concat_StrStr` "Received Damage: " (`KismetStringLibrary.Conv_DoubleToString` InDamage))))

(event `MulticastDamageReceived`
  (params (Instigator :type "Actor Object Reference") (Causer :type "Actor Object Reference") (Tags :type "GameplayTagContainer Structure") (Damage :type "Float (double-precision)"))
  (`|SpawnActorFromClass` "/Game/Blueprints/UI/Actors/BP_FloatingWidget.BP_FloatingWidget_C" (`KismetMathLibrary.MakeTransform` (+ (`self.K2_GetActorLocation`) (0.0 0.0 100.0))) "Undefined" "MultiplyWithRoot" null (`KismetTextLibrary.Conv_Int64ToText` (`KismetMathLibrary.Conv_DoubleToInt64` Damage)) null))

(fn `RotateTowardsMovement`
  (bind _returnvalue (`self.GetVelocity`))
  (bind _returnvalue_2 (`self.K2_GetActorLocation`))
  (if true
    (if (> (`KismetMathLibrary.VSize` _returnvalue) 0.0)
      (`self.K2_SetActorRotation` (`KismetMathLibrary.RInterpTo` (`self.K2_GetActorRotation`) (`KismetMathLibrary.FindLookAtRotation` _returnvalue_2 (+ (* _returnvalue (100.0 100.0 100.0)) _returnvalue_2)) (`GameplayStatics.GetWorldDeltaSeconds`) (`self.RotationSpeed`))))))

(fn `SetDragState`
  (params (bEnabled :type Boolean))
  (`self.SetMeshRelativeZState` bEnabled))

(fn `SetFocused`
  (params (bFocused :type Boolean))
  (bind _mesh (`self.Mesh`))
  (if bFocused
    (`KismetSystemLibrary.PrintString` "On Begin Cursor Over Skeletal Mesh")
    (`PrimitiveComponent.SetRenderCustomDepth` _mesh true)
    (`PrimitiveComponent.SetCustomDepthStencilValue` _mesh 250)
    (else
      (`PrimitiveComponent.SetRenderCustomDepth` _mesh false))))

(fn `SetMeshRelativeZState`
  (params (Dragged :type Boolean))
  (bind _mesh (`self.Mesh`))
  (`KismetSystemLibrary.PrintString` "Set Mesh Relative State")
  (if Dragged
    (`SceneComponent.K2_SetRelativeLocation` _mesh (`KismetMathLibrary.MakeVector` 0.0 0.0 200.0) false false)
    (else
      (`SceneComponent.K2_SetRelativeLocation` _mesh (`KismetMathLibrary.MakeVector` 0.0 0.0 -50.0) false false))))

(fn `SetupCosmetics`
  (bind _mesh (`self.Mesh`))
  (bind (_datatable _rowname) (break `DataTableRowHandle` (`self.UnitRow`)))
  (bind _returnvalue (`|GetDataTableRow` _datatable _rowname)
    (:`then`
      (bind (_unitid _unitname _uniticon _skeletalmesh _animinstance) (break `UnitData` _returnvalue))
      (`SkeletalMeshComponent.SetSkeletalMeshAsset` _mesh _skeletalmesh)
      (`SkeletalMeshComponent.SetAnimInstanceClass` _mesh _animinstance))))

(fn `SpawnNMAttProjectile`
  (params (OwnerUnit :type "BaseUnit Object Reference") (TargetUnit :type "BaseUnit Object Reference") (SpawnTransform :type "Transform Structure") (Instigator :type "Pawn Object Reference"))
  (bind _returnvalue (`|SpawnActorFromClass` "/Game/Blueprints/Projectiles/BP_BaseProjectile.BP_BaseProjectile_C" SpawnTransform "Undefined" "MultiplyWithRoot" null 50.0 0.0 Instigator))
  (set `BaseProjectile.OwnerUnit` OwnerUnit _returnvalue)
  (set `BaseProjectile.TargetUnit` TargetUnit _returnvalue))

(fn `UserConstructionScript`
  (`self.SetupCosmetics`))