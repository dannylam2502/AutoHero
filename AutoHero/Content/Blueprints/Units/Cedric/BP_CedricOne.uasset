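; Unit Blueprint for Cedric that relays his ultimate and Skill 1 hit events to the Gameplay Ability System.
; Each hit handler reads EnemyToAttack from the controller's blackboard and casts it to BP_BaseUnit.
; It then sends a skill-specific gameplay event to the instigator, with that enemy as target and target data.
; Construction only calls the parent script.
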(event `Handle Ultimate Hit`
  (bind _returnvalue (`self.GetInstigator`))
  (bind _asbp_base_unit (cast `/Game/Blueprints/Units/BP_BaseUnit` (`BlackboardComponent.GetValueAsObject` (`AIBlueprintHelperLibrary.GetBlackboard` (`self.GetController`)) "EnemyToAttack")))
  (`AbilitySystemBlueprintLibrary.SendGameplayEventToActor` _returnvalue (struct :`TagName` "char.cedric.ability.ultimate.hit") (make `GameplayEventData` (struct) _returnvalue _asbp_base_unit null null (struct) (struct) (struct) 0.0 (`AbilitySystemBlueprintLibrary.AbilityTargetDataFromActor` _asbp_base_unit))))

(event `Handle Skill 1 Hit`
  (bind _returnvalue (`self.GetInstigator`))
  (bind _asbp_base_unit (cast `/Game/Blueprints/Units/BP_BaseUnit` (`BlackboardComponent.GetValueAsObject` (`AIBlueprintHelperLibrary.GetBlackboard` (`self.GetController`)) "EnemyToAttack")))
  (`AbilitySystemBlueprintLibrary.SendGameplayEventToActor` _returnvalue (struct :`TagName` "CedricSkill1_Hit") (make `GameplayEventData` (struct) _returnvalue _asbp_base_unit null null (struct) (struct) (struct) 0.0 (`AbilitySystemBlueprintLibrary.AbilityTargetDataFromActor` _asbp_base_unit))))

(fn `UserConstructionScript`
  (`parent.UserConstructionScript`))