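; BP_Elara_One is an Elara unit Blueprint that supplies the projectile for the unit's normal attack.
; SpawnNMAttProjectile spawns a homing BP_ElaraProjectile_NormalAttack at the given transform's location with a fixed speed, passing the owner and target units.
; It then casts the result to BP_BaseProjectile and activates homing.
; The event graph holds only disabled placeholder events, and the construction script just calls the parent.
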(fn `SpawnNMAttProjectile`
  (params (OwnerUnit :type "BaseUnit Object Reference") (TargetUnit :type "BaseUnit Object Reference") (SpawnTransform :type "Transform Structure") (Instigator :type "Pawn Object Reference"))
  (bind _returnvalue (`self.SpawnProjectile` self "/Game/Blueprints/Projectiles/BP_ElaraProjectile_NormalAttack.BP_ElaraProjectile_NormalAttack_C" (.location SpawnTransform) (struct) 700.0 0.0 true OwnerUnit TargetUnit))
  (bind _asbp_base_projectile (cast `/Game/Blueprints/Projectiles/BP_BaseProjectile` _returnvalue))
  (`/Game/Blueprints/Projectiles/BP_BaseProjectile.Activate Homing Target` _asbp_base_projectile))

(fn `UserConstructionScript`
  (`parent.UserConstructionScript`))