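; Player controller that lets the player hover, drag and drop BP_BaseUnit pawns to place them on the field.
; Each Tick, a cursor trace against Pawns updates the focused unit, except while dragging.
; Left mouse press starts dragging the focused unit, which then follows the cursor's WorldStatic hit point.
; Release finalizes placement and resets the drag, with unit state set at both ends.
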(event `self.ReceiveTick`
  (params (DeltaSeconds :type "Float (single-precision)"))
  (`parent.ReceiveTick` DeltaSeconds)
  (`self.FindFocusedUnit`)
  (if (`self.bDragging`)
    (`self.UpdateDraggedUnitLocation`)))

(event `Key|LeftMouseButton`
  (params (Key :type "Key Structure"))
  (:`Pressed`
    (`self.HasFocusedUnit`
      (:`Valid`
        (if (not (`self.bDragging`))
          (`self.StartDragging` (`self.FocusedUnit`))))))
  (:`Released`
    (`/Engine/EditorBlueprintResources/StandardMacros.IsValid` (`self.DraggingUnit`)
      (:`Is Valid`
        (`BaseUnit.FinalizePlacement` (`self.DraggingUnit`))
        (`self.StopDragging`)))))

(event `self.ReceiveBeginPlay`
  (`EnhancedInputSubsystemInterface.AddMappingContext` (pcsubsystem `EnhancedInputLocalPlayerSubsystem` (`GameplayStatics.GetPlayerController` 0)) "/Game/Blueprints/Inputs/IMC_Default.IMC_Default" 0 (struct)))

(fn `FindFocusedUnit`
  (bind (_bblockinghit _binitialoverlap _time _distance _location _impactpoint _normal _impactnormal _physmat _hitactor) (`GameplayStatics.BreakHitResult` (`self.GetHitResultUnderCursorForObjects` (`|MakeArray` "ObjectTypeQuery3" :!type "EObjectTypeQuery Enum"))))
  (set `self.CursorLocation` _location)
  (if (not (`self.bDragging`))
    (`/Engine/EditorBlueprintResources/StandardMacros.IsValid` _hitactor
      (:`Is Valid`
        (if (!= _hitactor (`self.FocusedUnit`))
          (bind _asbp_base_unit (cast `/Game/Blueprints/Units/BP_BaseUnit` _hitactor)
            (:`then`
              (`self.UnfocusUnit`)
              (`self.SetFocusedUnit` _asbp_base_unit))
            (:`CastFailed`
              (`self.UnfocusUnit` :!label _label)))))
      (:`Is Not Valid`
        (goto _label)))))

(fn `GetFocusedUnit`
  (returns (ReturnValue :type "/Game/Blueprints/Units/BP_BaseUnit Object Reference"))
  (return (`self.FocusedUnit`)))

(fn `SetFocusedUnit`
  (params (InUnit :type "/Game/Blueprints/Units/BP_BaseUnit Object Reference"))
  (`/Engine/EditorBlueprintResources/StandardMacros.IsValid` InUnit
    (:`Is Valid`
      (bind _output_get (set `self.FocusedUnit` InUnit))
      (`/Game/Blueprints/Units/BP_BaseUnit.SetFocused` _output_get true))))

(fn `StartDragging`
  (params (UnitToDrag :type "/Game/Blueprints/Units/BP_BaseUnit Object Reference"))
  (bind _output_get (set `self.DraggingUnit` UnitToDrag))
  (`BaseUnit.SetUnitState` _output_get "DraggingInField")
  (set `self.bDragging` true))

(fn `StopDragging`
  (bind _null (`self.Null`))
  (`BaseUnit.SetUnitState` (`self.DraggingUnit`) "WaitingForPlacement")
  (set `self.bDragging` false)
  (set `self.FocusedUnit` _null)
  (set `self.DraggingUnit` _null))

(fn `UnfocusUnit`
  (bind _focusedunit (`self.FocusedUnit`))
  (`/Engine/EditorBlueprintResources/StandardMacros.IsValid` _focusedunit
    (:`Is Valid`
      (`/Game/Blueprints/Units/BP_BaseUnit.SetFocused` _focusedunit false)
      (set `self.FocusedUnit` null))))

(fn `UpdateDraggedUnitLocation`
  (bind _draggingunit (`self.DraggingUnit`))
  (`/Engine/EditorBlueprintResources/StandardMacros.IsValid` _draggingunit
    (:`Is Valid`
      (`self.K2_SetActorLocation` _draggingunit (`.Location` (`GameplayStatics.BreakHitResult` (`self.GetHitResultUnderCursorForObjects` (`|MakeArray` "ObjectTypeQuery1" :!type "EObjectTypeQuery Enum")))) false false))))

(fn `UserConstructionScript`)