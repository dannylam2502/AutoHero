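; Cocu's Healing Bell gameplay ability, which launches a healing bell projectile at every unit on the caster's team.
; On a successful commit it plays a montage and waits once for the Char.cocu.healingbell gameplay event.
; On that event, GetAllyList filters all BaseUnit actors by team, caster included, and the caster spawns one targeted projectile per result.
; EndAbility is called only when the commit fails.
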(event `self.K2_ActivateAbility`
  (bind _ownerunit (`self.OwnerUnit`))
  ;[1 1 1] Template Block
  (bind _returnvalue (`self.K2_CommitAbility`))
  (if _returnvalue
    (bind _outmontagetoplay (`self.GetMontageToPlay`))
    (`AbilityTask_PlayMontageAndWait.CreatePlayMontageAndWaitProxy` "None" _outmontagetoplay
      (:`then`
        (bind _asynctaskproxy (`AbilityTask_WaitGameplayEvent.WaitGameplayEvent` (struct :`TagName` "char.cocu.healingbell") null true)
          (:`then`
            (set `self.Async Task` _asynctaskproxy))
          (:`EventReceived`
            (bind _asbase_unit (cast `BaseUnit` (`self.GetOwningActorFromActorInfo`))
              (:`then`
                (set `self.OwnerUnit` _asbase_unit)
                (bind _baseunits (`self.GetAllyList` (`BaseUnit.ETeam` _asbase_unit)))
                (for _index (range (`KismetArrayLibrary.Array_Length` _baseunits))
                  (`BaseUnit.SpawnProjectile` :`self` _ownerunit :`WorldContextObject` _ownerunit :`BPProjectile` "/Game/Blueprints/Projectiles/BP_CocuProjectile_HealingBell.BP_CocuProjectile_HealingBell_C" :`InOwnerUnit` _ownerunit :`InTargetUnit` (`|GetArrayItem` _baseunits _index))))
              (:`CastFailed`
                (`KismetSystemLibrary.PrintString` "CAST FAILED!!" true true (struct :`R` 1.0 :`B` 0.023943 :`A` 1.0))))))))
    (else
      (`self.K2_EndAbility`))))

(fn `GetAllyList`
  (params (Team :type "EActorTeam Enum" :default "Blue"))
  (returns (BaseUnits :type "Array of BaseUnit Object Reference"))
  (locals (ReturnList :type "Array of BaseUnit Object Reference"))
  (bind _returnlist (`local.ReturnList`))
  (bind _outactors (`GameplayStatics.GetAllActorsOfClass` "/Script/AutoHero.BaseUnit"))
  (for _array_element _outactors
    (if (== (`BaseUnit.ETeam` _array_element) (`KismetMathLibrary.Conv_ByteToInt64` Team))
      (`KismetArrayLibrary.Array_Add` _returnlist _array_element)))
  (return _returnlist))